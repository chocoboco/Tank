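; Tank_BP is a player-controllable tank that routes input to its aiming and movement components and drives an orbit camera.
; On BeginPlay it hands the barrel and turret to TankAiming and the two tracks to TankMovement.
; Axis inputs rotate the azimuth gimbal and spring arm or set movement intents, while Fire calls TankAiming.
; It also passes itself to the HealthBar_BP widget so the bar can reference the tank.
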(event EventBeginPlay
  (Class|TankAimingComponent|Initalize (Variables|Default|GetTankAiming) (Variables|Default|GetBarrel) (Variables|Default|GetTurret))
  (Class|TankMovementComponent|Initialize (Variables|Default|GetTankMovement) (Variables|Default|GetLeft%20Track) (Variables|Default|GetRight%20Track))
  (CallFunction|SetTankBPReftoHealthBarWidget))

(event Collision|EventActorBeginOverlap
  (params (OtherActor :type Actor%20Object%20Reference)))

(event EventTick
  (params (DeltaSeconds :type Float%20%28single-precision%29)))

(event Input|ActionEvents|InputActionFire
  (params (Key :type Key%20Structure))
  ;[1 1 1] Camera Input Binding
  (:Pressed
    (Class|TankAimingComponent|Fire (Variables|Default|GetTankAiming))))

(event Input|AxisEvents|InputAxisTurnRight
  (params (AxisValue :type Float%20%28single-precision%29))
  ;[1 1 1] Camera Input Binding
  (Class|TankMovementComponent|IntendTurnRight (Variables|Default|GetTankMovement) AxisValue))

(event Input|AxisEvents|InputAxisAimAzimuth
  (params (AxisValue :type Float%20%28single-precision%29))
  ;[1 1 1] Camera Input Binding
  (Transformation|AddLocalRotation (Variables|Default|GetAzimuth%20Gimbal) (Math|Rotator|MakeRotator 0.0 0.0 AxisValue) false false))

(event Input|AxisEvents|InputAxisMoveForward
  (params (AxisValue :type Float%20%28single-precision%29))
  ;[1 1 1] Camera Input Binding
  (Class|TankMovementComponent|IntendMoveForward (Variables|Default|GetTankMovement) AxisValue))

(event Input|AxisEvents|InputAxisAimElevation
  (params (AxisValue :type Float%20%28single-precision%29))
  ;[1 1 1] Camera Input Binding
  (Transformation|AddLocalRotation (Variables|Default|GetSpringArm) (Math|Rotator|MakeRotator 0.0 AxisValue 0.0) false false))

(fn ConstructionScript)

(fn SetTankBPReftoHealthBarWidget
  (bind _ashealth_bar_bp (Utilities|Casting|CastToHealthBar_BP (UserInterface|GetUserWidgetObject (Variables|Default|GetHealth%20Bar%20Widget)))
    (:then
      (Variables|/Game/UI/HealthBar_BP.HealthBar_BP_C|SetTankRef _ashealth_bar_bp self)
      (return))
    (:CastFailed
      (Development|PrintString "HealthBar_BP Set Failed!!"))))